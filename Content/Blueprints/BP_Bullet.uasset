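; BP_Bullet is a bullet actor that explodes on contact and cleans itself up.
; On BeginPlay a timer destroys it after a few seconds if nothing is hit.
; Any overlap on its Box component spawns a scaled-down explosion particle and sound at its location, then destroys it.
; The graph applies no damage, and a Player tag check is left unconnected.
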(event `self.ReceiveBeginPlay`
  (`KismetSystemLibrary.K2_SetTimerDelegate` (delegate `DestroySelf`) 3.0))

(event `DestroySelf`
  (`self.K2_DestroyActor`))

(event `self.Box.OnComponentBeginOverlap`
  (params (OverlappedComponent :type "PrimitiveComponent Object Reference") (OtherActor :type "Actor Object Reference") (OtherComp :type "PrimitiveComponent Object Reference") (OtherBodyIndex :type Integer) (bFromSweep :type Boolean) (SweepResult :type "HitResult Structure (by ref)"))
  (`GameplayStatics.SpawnEmitterAtLocation` "/Game/StarterContent/Particles/P_Explosion.P_Explosion" (`self.K2_GetActorLocation`) (`self.K2_GetActorRotation`) (0.2 0.2 0.2))
  (`GameplayStatics.SpawnSoundAtLocation` "/Game/StarterContent/Audio/Explosion_Cue.Explosion_Cue" (`self.K2_GetActorLocation`))
  (`self.K2_DestroyActor`))

(fn `UserConstructionScript`)