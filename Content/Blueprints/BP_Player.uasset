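; BP_Player is the player-controlled propeller aircraft, which flies forward constantly and shoots bullets.
; Tick spins both propellers and applies forward movement input scaled by BoosterValue, which the Booster action raises while held.
; Roll and Pitch axes apply frame-rate-independent local rotations, with roll also scaled by the boost value.
; Two Fire handlers spawn BP_Bullet at separate arrow components, while the Accel axis is left empty.
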(event `InputAction|Booster`
  (params (Key :type "Key Structure"))
  (:`Pressed`
    (set `self.BoosterValue` 1.0))
  (:`Released`
    (set `self.BoosterValue` 0.3)))

(event `InputAxis|Roll`
  (params (AxisValue :type "Float (single-precision)"))
  (`self.K2_AddActorLocalRotation` (`KismetMathLibrary.MakeRotator` (* AxisValue (`GameplayStatics.GetWorldDeltaSeconds`) (`self.RotateSpeed`) (`self.BoosterValue`)))))

(event `self.ReceiveTick`
  (params (DeltaSeconds :type "Float (single-precision)"))
  (`|ExecutionSequence`
    (:`then_0`
      (`self.RotatePropeller` (`self.Propeller_L`)))
    (:`then_1`
      (`self.RotatePropeller` (`self.Propeller_R`)))
    (:`then_2`
      (`self.AddMovementInput` (`self.GetActorForwardVector`) (`self.BoosterValue`)))))

(event `InputAxis|Pitch`
  (params (AxisValue :type "Float (single-precision)"))
  (`self.K2_AddActorLocalRotation` (`KismetMathLibrary.MakeRotator` 0.0 (* AxisValue (`GameplayStatics.GetWorldDeltaSeconds`) (`self.RotateSpeed`) -1.0))))

(event `RotatePropeller`
  (params (Propeller :type "StaticMeshComponent Object Reference"))
  (`SceneComponent.K2_AddLocalRotation` Propeller (`KismetMathLibrary.MakeRotator` 0.0 0.0 (* (`self.PropellerRotate`) (`GameplayStatics.GetWorldDeltaSeconds`))) false false))

(event `InputAxis|Accel`
  (params (AxisValue :type "Float (single-precision)")))

(event `InputAction|Fire`
  (params (Key :type "Key Structure"))
  (:`Pressed`
    (`|SpawnActorFromClass` "/Game/Blueprints/BP_Bullet.BP_Bullet_C" (`SceneComponent.K2_GetComponentToWorld` (`self.Arrow1`)) "Undefined" "OverrideRootScale" null null)))

(event `InputAction|Fire`
  (params (Key :type "Key Structure"))
  (:`Pressed`
    (`|SpawnActorFromClass` "/Game/Blueprints/BP_Bullet.BP_Bullet_C" (`SceneComponent.K2_GetComponentToWorld` (`self.Arrow2`)) "Undefined" "OverrideRootScale" null null)))

(fn `UserConstructionScript`)